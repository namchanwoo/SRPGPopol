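; Player pawn for grid-based battles, providing a camera that moves relative to control yaw, turns while right-click is held, and zooms via clamped spring arm length.
; Enhanced Input events drive it, with primary-click release ending deployment drags through the Grid's battle controller.
; Right-click also cancels the active ability or spell.
; A gate with a short delay detects double right-clicks to restore the initial rotation.
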(event Custom|DoubleRightClick
  (Utilities|FlowControl|Sequence
    (:then_0
      (Utilities|FlowControl|Gate true :!label _label
        (:Exit
          (Pawn|SetControlRotation (Game|GetPlayerController 0) (Variables|Default|GetInitialRotation)))))
    (:then_1
      (goto _label Open))
    (:then_2
      (Utilities|FlowControl|Delay 0.2)
      (goto _label Close))))

(event Input|EnhancedActionEvents|EnhancedInputActionIA_Move
  (params (ActionValue :type Vector%202D%20Structure) (ElapsedSeconds :type Float%20%28double-precision%29) (TriggeredSeconds :type Float%20%28double-precision%29) (InputAction :type Input%20Action%20Object%20Reference :default "/Game/Game_/Input/IA_Move.IA_Move"))
  (bind _returnvalue (Pawn|GetControlRotation :!class /Script/Engine.Pawn))
  (bind _yaw (Math|Rotator|BreakRotator _returnvalue))
  (bind _returnvalue_2 (Math|Rotator|MakeRotator 0.0 0.0 _yaw))
  (:Triggered
    (Pawn|Input|AddMovementInput (Math|Vector|GetForwardVector _returnvalue_2) (.y ActionValue) false)
    (Pawn|Input|AddMovementInput (Math|Vector|GetRightVector _returnvalue_2) (.x ActionValue) false)))

(event Input|EnhancedActionEvents|EnhancedInputActionIA_PrimaryClick
  (params (ActionValue :type Boolean) (ElapsedSeconds :type Float%20%28double-precision%29) (TriggeredSeconds :type Float%20%28double-precision%29) (InputAction :type Input%20Action%20Object%20Reference :default "/Game/Game_/Input/IA_PrimaryClick.IA_PrimaryClick"))
  (:Completed
    (Class|DeploymentController|OnDragEnded (Variables|/Script/SRG.BattleController|GetDeploymentController (Variables|/Script/SRG.Grid|GetBattleControllerRef (Variables|Default|GetGrid))))))

(event Input|EnhancedActionEvents|EnhancedInputActionIA_Secondaryclick
  (params (ActionValue :type Boolean) (ElapsedSeconds :type Float%20%28double-precision%29) (TriggeredSeconds :type Float%20%28double-precision%29) (InputAction :type Input%20Action%20Object%20Reference :default "/Game/Game_/Input/IA_Secondaryclick.IA_Secondaryclick"))
  (bind _grid (Variables|Default|GetGrid))
  (bind _battlecontrollerref (Variables|/Script/SRG.Grid|GetBattleControllerRef _grid))
  (:Started
    (Class|BattleController|PlayerCancelActiveAbility _battlecontrollerref)
    (Class|BattleController|CancelSpell _battlecontrollerref)
    (CallFunction|DoubleRightClick)
    (Utilities|FlowControl|Gate true) ; enters at Open
  )
  (:Completed
    (Utilities|FlowControl|Gate true) ; enters at Close
  ))

(event Input|EnhancedActionEvents|EnhancedInputActionIA_Turn
  (params (ActionValue :type Float%20%28double-precision%29) (ElapsedSeconds :type Float%20%28double-precision%29) (TriggeredSeconds :type Float%20%28double-precision%29) (InputAction :type Input%20Action%20Object%20Reference :default "/Game/Game_/Input/IA_Turn.IA_Turn"))
  (:Triggered
    (Utilities|FlowControl|Gate true
      (:Exit
        (Pawn|Input|AddControllerYawInput ActionValue)))))

(event Input|EnhancedActionEvents|EnhancedInputActionIA_Zoom
  (params (ActionValue :type Float%20%28double-precision%29) (ElapsedSeconds :type Float%20%28double-precision%29) (TriggeredSeconds :type Float%20%28double-precision%29) (InputAction :type Input%20Action%20Object%20Reference :default "/Game/Game_/Input/IA_Zoom.IA_Zoom"))
  (:Triggered
    (Variables|Default|SetTargetZoom (Math|Float|Clamp(Float) (+ (* ActionValue -6e+01) (Variables|Default|GetTargetZoom)) (Variables|Default|GetMinZoom) (Variables|Default|GetMaxZoom)))
    (Variables|/Script/Engine.SpringArmComponent|SetTargetArmLength (Variables|Default|GetSpringArm) (Variables|Default|GetTargetZoom))))

(event EventBeginPlay
  (Variables|Default|SetInitialRotation (Pawn|GetControlRotation (Game|GetPlayerController 0) :!class /Script/Engine.Controller))
  (bind _returnvalue (Actor|GetActorOfClass "/Script/SRG.Grid"))
  (Variables|Default|SetGrid _returnvalue)
  (Input|AddMappingContext (PlayerController|LocalPlayerSubsystems|GetEnhancedInputLocalPlayerSubsystem (Game|GetPlayerController 0)) "/Game/Game_/Input/IMC_SRG_Default.IMC_SRG_Default" 0 "(bIgnoreAllPressedKeysUntilRelease=True,bForceImmediately=False)"))

(fn ConstructionScript)