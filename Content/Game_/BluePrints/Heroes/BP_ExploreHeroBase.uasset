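; Base Blueprint for explore heroes, providing click-to-move toward the point under the cursor.
; While input is not blocked, the primary click traces the Visibility channel, then moves via SimpleMoveToLocation and calls ShowPath if the hit is far enough from the hero.
; When ContinuousMovement is set, the ContinuosMove timeline's Move event re-runs the same logic until the click completes.
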(event EventBeginPlay)

(event Collision|EventActorBeginOverlap
  (params (OtherActor :type Actor%20Object%20Reference)))

(event EventTick
  (params (DeltaSeconds :type Float%20%28single-precision%29)))

(event Input|EnhancedActionEvents|EnhancedInputActionIA_PrimaryClick
  (params (ActionValue :type Boolean) (ElapsedSeconds :type Float%20%28double-precision%29) (TriggeredSeconds :type Float%20%28double-precision%29) (InputAction :type Input%20Action%20Object%20Reference :default "/Game/Game_/Input/IA_PrimaryClick.IA_PrimaryClick"))
  (bind _returnvalue (Game|GetPlayerController 0))
  (bind (_hitresult _returnvalue_2) (Game|Player|GetHitResultUnderCursorbyChannel _returnvalue "TraceTypeQuery1" true))
  (bind _location (Collision|BreakHitResult _hitresult))
  ;[1 0 0.3281] IA_PrimartClick
  (:Triggered
    (Class|ExploreHeroBase|CheckMovement)
    (Utilities|IsEnputInabled
      (:Enabled
        (if _returnvalue_2
          (if (>= (Math|Vector|VectorLength (- (Transformation|GetActorLocation) _location)) 1e+02)
            (AI|Navigation|SimpleMovetoLocation (Game|GetPlayerController 0) _location)
            (Class|ExploreHeroBase|ShowPath _location))))))
  (:Completed
    (Class|ExploreHeroBase|StopCheckingMovement)))

(event EventCheckMovement
  (bind _returnvalue (Game|GetPlayerController 0))
  (bind (_hitresult _returnvalue_2) (Game|Player|GetHitResultUnderCursorbyChannel _returnvalue "TraceTypeQuery1" true))
  (bind _location (Collision|BreakHitResult _hitresult))
  ;[1 0 0.3281] IA_PrimartClick
  (if (Variables|Default|GetbContinuousMovement)
    (Timeline|ContinuosMove PlayFromStart
      (:Move
        (Utilities|IsEnputInabled
          (:Enabled
            (if _returnvalue_2
              (if (>= (Math|Vector|VectorLength (- (Transformation|GetActorLocation) _location)) 1e+02)
                (AI|Navigation|SimpleMovetoLocation (Game|GetPlayerController 0) _location)
                (Class|ExploreHeroBase|ShowPath _location)))))))))

(event EventStopCheckingMovement
  (bind _returnvalue (Game|GetPlayerController 0))
  (bind (_hitresult _returnvalue_2) (Game|Player|GetHitResultUnderCursorbyChannel _returnvalue "TraceTypeQuery1" true))
  (bind _location (Collision|BreakHitResult _hitresult))
  ;[1 0 0.3281] IA_PrimartClick
  (Timeline|ContinuosMove Stop
    (:Move
      (Utilities|IsEnputInabled
        (:Enabled
          (if _returnvalue_2
            (if (>= (Math|Vector|VectorLength (- (Transformation|GetActorLocation) _location)) 1e+02)
              (AI|Navigation|SimpleMovetoLocation (Game|GetPlayerController 0) _location)
              (Class|ExploreHeroBase|ShowPath _location))))))))

(fn ConstructionScript)