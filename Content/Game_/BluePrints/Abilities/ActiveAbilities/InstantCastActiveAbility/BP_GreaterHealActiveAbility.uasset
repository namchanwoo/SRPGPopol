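; Instant-cast active ability for a greater heal in a turn-based game with slot-based targeting.
; On use, it heals every ally in range by a fixed amount, then ends the turn.
; Its AI check approves the ability when any ally in range is missing at least half that heal amount in health.
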(event EventOnAbilityUsed
  (params (InSlotsInRange :type Array%20of%20Slot%20Base%20Object%20References) (InEmptySlotsInRange :type Array%20of%20Slot%20Base%20Object%20References) (InAlliesInRange :type Array%20of%20Character%20Base%20Object%20References) (InEnemiesInRange :type Array%20of%20Character%20Base%20Object%20References))
  (for _array_element InAlliesInRange
    (Class|CharacterBase|Heal _array_element 50))
  (Class|ActiveAbilityBase|EndTurn))

(fn ConstructionScript)

(fn ShouldAIUse
  (params (SlotsInRange :type Array%20of%20Slot%20Base%20Object%20References) (EmptySlotsInRange :type Array%20of%20Slot%20Base%20Object%20References) (AlliesInRange :type Array%20of%20Character%20Base%20Object%20References) (EnemiesInRange :type Array%20of%20Character%20Base%20Object%20References) (WeakestEnemy :type Character%20Base%20Object%20Reference))
  (for _array_element AlliesInRange
    (if (>= (- (.maxhealth (Variables|/Script/SRG.CharacterBase|GetCharacterStats _array_element)) (Variables|/Script/SRG.CharacterBase|GetCurrentHealth _array_element)) 25)
      (LocalVariables|SetCurrentShouldAIUse true)))
  (return (LocalVariables|GetCurrentShouldAIUse)))