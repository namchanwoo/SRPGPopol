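; Fireball active area-target ability that damages enemies within range of a targeted slot and then ends the turn.
; On use it builds fixed elemental damage data per enemy and launches a fireball actor at the slot from an elevated offset.
; Damage, the parent ability logic and turn end wait for the projectile's hit event.
; For AI targeting, it picks a random opposing character's slot.
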(event Custom|OnFireballHit
  (EventDispatchers|UnbindEventfromOnProjectileHit (stale EventOnAbilityUsed _returnvalue_3) (delegate Custom|OnFireballHit))
  (Class|ActiveAbilityBase|DamageTargets (stale EventOnAbilityUsed _returnvalue_2))
  (|CallParentFunction (stale EventOnAbilityUsed InSlotsInRange) (stale EventOnAbilityUsed InEmptySlotsInRange) (stale EventOnAbilityUsed InAlliesInRange) (stale EventOnAbilityUsed InEnemiesInRange))
  (Class|ActiveAbilityBase|EndTurn))

(event EventSetTargetSlotforAI
  (Variables|Default|SetTargetSlot (Variables|/Script/SRG.UnitBase|GetSlot (.OutItem (Utilities|Array|Random (select (Variables|/Script/SRG.CharacterBase|GetbIsAI (Variables|Default|GetAbilityOwner)) (Variables|/Script/SRG.BattleController|GetPlayerCharacters (Variables|Default|GetBattleController)) (Variables|/Script/SRG.BattleController|GetEnemyCharacters (Variables|Default|GetBattleController))))))))

(event EventOnAbilityUsed
  (params (InSlotsInRange :type Array%20of%20Slot%20Base%20Object%20References) (InEmptySlotsInRange :type Array%20of%20Slot%20Base%20Object%20References) (InAlliesInRange :type Array%20of%20Character%20Base%20Object%20References) (InEnemiesInRange :type Array%20of%20Character%20Base%20Object%20References))
  (bind _targetslot (Variables|Default|GetTargetSlot))
  (bind _returnvalue (Transformation|GetActorLocation _targetslot))
  (bind _returnvalue_2 (CallFunction|GetAbilityDamage InEnemiesInRange))
  (bind _returnvalue_3 (Game|SpawnActorfromClass "/Game/Game_/BluePrints/Projectiles/BP_FireBall.BP_FireBall_C" (Math|Transform|MakeTransform (+ _returnvalue (Math|Vector|MakeVector -4e+02 0.0 6e+02)) "0, 0, 0" "1.000000,1.000000,1.000000") "Undefined" 0 0))
  (Default|MoveProjectiletoTarget _returnvalue_3 _returnvalue)
  (EventDispatchers|BindEventtoOnProjectileHit _returnvalue_3 (delegate Custom|OnFireballHit)))

(fn ConstructionScript)

(fn GetAbilityDamage
  (params (InTargetCharacters :type Array%20of%20Character%20Base%20Object%20References))
  (for _array_element InTargetCharacters
    (Utilities|Map|Add (LocalVariables|GetCurrentDamageData) _array_element (Utilities|Struct|MakeDamageData 25 25 25 1.0 (Variables|Default|GetElement))))
  (return (LocalVariables|GetCurrentDamageData)))