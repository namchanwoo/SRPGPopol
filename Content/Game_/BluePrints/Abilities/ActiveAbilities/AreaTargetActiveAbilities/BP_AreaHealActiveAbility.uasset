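; An area-target active ability for turn-based battles that heals allies in range.
; On use, it calls Heal on every ally passed in with an amount of zero, then ends the turn.
; For AI targeting, it scans the owner's side through the BattleController and targets the slot of the first character missing at least a fixed amount of health.
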(event EventOnAbilityUsed
  (params (InSlotsInRange :type Array%20of%20Slot%20Base%20Object%20References) (InEmptySlotsInRange :type Array%20of%20Slot%20Base%20Object%20References) (InAlliesInRange :type Array%20of%20Character%20Base%20Object%20References) (InEnemiesInRange :type Array%20of%20Character%20Base%20Object%20References))
  (for _array_element InAlliesInRange
    (Class|CharacterBase|Heal _array_element))
  (Class|ActiveAbilityBase|EndTurn))

(event EventSetTargetSlotforAI
  (bind _battlecontroller (Variables|Default|GetBattleController))
  (bind _array_element (Utilities|Array|ForEachLoopwithBreak (select (Variables|/Script/SRG.CharacterBase|GetbIsAI (Variables|Default|GetAbilityOwner)) (Variables|/Script/SRG.BattleController|GetEnemyCharacters _battlecontroller) (Variables|/Script/SRG.BattleController|GetPlayerCharacters _battlecontroller)) :!label _label)
    (:LoopBody
      (if (>= (- (.maxhealth (Variables|/Script/SRG.CharacterBase|GetMainStats _array_element)) (Variables|/Script/SRG.CharacterBase|GetCurrentHealth _array_element)) 25)
        (Class|ActiveAbilityBase|SetTargetSlot (Variables|/Script/SRG.UnitBase|GetSlot _array_element))
        (goto _label Break)))))

(fn ConstructionScript)