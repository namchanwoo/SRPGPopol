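; BP_ProjectileSplashPassiveAbility is a multi-target passive ability that selects splash victims around the attacked slot on the battle grid.
; GetEnemiesInAbilityRange asks the BattleController's Grid for slots within Range of the attack slot, occupied ones included, and ignores the standing slot.
; It rebuilds EnemyCharacters from unique enemies of AbilityOwner in those slots and returns it; the event graph holds no logic.
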(event EventBeginPlay)

(event EventTick
  (params (DeltaSeconds :type Float%20%28single-precision%29)))

(fn ConstructionScript)

(fn GetEnemiesinAbilityRange
  (params (InAttackSlot :type Slot%20Base%20Object%20Reference) (InStandingSlot :type Slot%20Base%20Object%20Reference))
  ;[1 0.8906 0] 대상 슬롯 주변의 적을 되돌립니다.
  ; 범위 1 = 대상 슬롯
  ; 범위 3 = 대상 슬롯 및 인접 슬롯
  (Utilities|Array|Clear (Variables|Default|GetEnemyCharacters))
  (bind _outslotsinrange (Class|Grid|GetSlotsinRange (Variables|/Script/SRG.BattleController|GetGrid (Variables|Default|GetBattleController)) InAttackSlot (Variables|Default|GetRange) false))
  (for _array_element _outslotsinrange
    (if (.ReturnValue (Class|SlotBase|IsEnemySlot _array_element (Variables|Default|GetAbilityOwner)))
      (Utilities|Array|AddUnique (Variables|Default|GetEnemyCharacters) (.OutEnemyCharacter (Class|SlotBase|IsEnemySlot _array_element (Variables|Default|GetAbilityOwner))))))
  (return (Variables|Default|GetEnemyCharacters)))