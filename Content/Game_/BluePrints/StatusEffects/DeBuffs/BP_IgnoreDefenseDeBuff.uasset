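; BP_IgnoreDefenseDeBuff is a status effect debuff that strips the affected character's defense for as long as it lasts.
; On start it stores the character's current defense and applies its negation through ApplyStats, leaving all other stats unchanged.
; On end it adds the stored amount back and destroys its own actor.
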(event EventOnStatusEffectStarted
  (Variables|Default|SetinitialDefense (Variables|/Script/SRG.CharacterBase|GetCurrentDefense (Variables|Default|GetAffectedCharacter)))
  (Class|CharacterBase|ApplyStats (Variables|Default|GetAffectedCharacter) (Utilities|Struct|MakeCharacterStats 0 0 0 (* (Variables|Default|GetinitialDefense) -1) 0 0 0 0)))

(event EventOnStatusEffectEnded
  (Class|CharacterBase|ApplyStats (Variables|Default|GetAffectedCharacter) (Utilities|Struct|MakeCharacterStats 0 0 0 (Variables|Default|GetinitialDefense) 0 0 0 0))
  (Actor|DestroyActor))

(fn ConstructionScript)