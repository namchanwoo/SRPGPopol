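; Poison debuff status effect that deals Earth-element damage over time to the affected character and reports Earth as its UI element.
; Each DOT tick takes a fraction of max health, rounds it up, applies elemental reductions and sends it through the character's damage event.
; It then calls OnDOTApplied with the hit montage length plus a short buffer, or zero when no montage exists.
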(event EventOnDOT
  (Class|CharacterBase|TakeDamageEvent (Variables|Default|GetAffectedCharacter) (Class|StatusEffectBase|GetDamageAfterElementReductions (Math|Float|Ceil (* (.MaxHealth (Utilities|Struct|BreakCharacterStats (Variables|/Script/SRG.CharacterBase|GetMainStats (Variables|Default|GetAffectedCharacter)))) (Variables|StatusEffect|GetDOTAmount))) "Earth") "Earth")
  (bind _gethitmontage (Variables|/Script/SRG.CharacterBase|GetGetHitMontage (Variables|Default|GetAffectedCharacter))
    (:then
      (Default|CallOnDOTApplied (+ (Variables|/Script/Engine.AnimSequenceBase|GetSequenceLength _gethitmontage) 0.5)))
    (:else
      (Default|CallOnDOTApplied 0.0))))

(fn ConstructionScript)

(fn ShowElementonUI
  (return "Earth"))