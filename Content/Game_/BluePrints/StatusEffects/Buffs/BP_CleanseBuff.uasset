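; BP_CleanseBuff is a status effect buff that strips debuffs from the affected character.
; On initialization it walks the character's current debuffs in reverse, so entries can be removed during the loop, and removes each one that does not come from an aura.
; It skips all removal if the cleanse itself comes from an aura.
; It then removes itself immediately, acting as an instant one-shot effect.
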(event EventInitializeEvent
  (bind _arrayelement (Utilities|Array|ReverseforEachLoop (Variables|/Script/SRG.CharacterBase|GetCurrentDeBuffs (Variables|Default|GetAffectedCharacter)))
    (:LoopBody
      (if (and (not (Variables|/Script/SRG.StatusEffectBase|GetbIsFromAura _arrayelement)) (not (Variables|Default|GetbIsFromAura)))
        (Class|StatusEffectBase|RemoveStatusEffect _arrayelement)))
    (:Completed
      (Class|StatusEffectBase|RemoveStatusEffect))))

(fn ConstructionScript)